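; Melee enemy Blueprint that carries a greatsword, built on a parent enemy class whose weapon events it extends.
; Attach and Detach move the GreatSword component between the hand and holster sockets on the mesh and set the Attached flag.
; Equipped and Unequipped set or clear the current weapon and switch the CombatType enum.
; Each override calls its parent implementation first, while BeginPlay, overlap and construction add no logic of their own.
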(event EventBeginPlay
  (|CallParentFunction) ; 지금 이 노드는 비활성 상태입니다. \n핀을 끌어서 다른 노드를 연결하면 활성화됩니다.
)

(event Collision|EventActorBeginOverlap
  (params (OtherActor :type Actor%20Object%20Reference))
  (|CallParentFunction OtherActor) ; 지금 이 노드는 비활성 상태입니다. \n핀을 끌어서 다른 노드를 연결하면 활성화됩니다.
)

(event EventAttach
  (|CallParentFunction)
  (Transformation|AttachComponentToComponent (Variables|Default|GetGreatSword) (Variables|Character|GetMesh) "Hand_GreatSword" "KeepRelative" "KeepRelative" "KeepRelative" true)
  (Variables|Default|SetAttached true))

(event EventDetach
  (|CallParentFunction)
  (Transformation|AttachComponentToComponent (Variables|Default|GetGreatSword) (Variables|Character|GetMesh) "Holster_GreatSword" "KeepRelative" "KeepRelative" "KeepRelative" true)
  (Variables|Default|SetAttached false))

(event EventEquipped
  (|CallParentFunction)
  (CallFunction|SetCurrentWeapon (Variables|Default|GetGreatSword))
  (Variables|Default|SetCombatType "NewEnumerator1"))

(event EventUnequipped
  (|CallParentFunction)
  (CallFunction|SetCurrentWeapon)
  (Variables|Default|SetCombatType "NewEnumerator0"))

(fn ConstructionScript
  (|CallParentFunction))